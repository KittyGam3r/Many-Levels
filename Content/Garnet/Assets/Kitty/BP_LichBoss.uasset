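; Lich boss enemy that, while activated, chases a minion if the player's MinionCount is above zero, otherwise the player.
; Touching a minion kills it and decrements that count; touching either minion or player deactivates the boss and leads to opening Jennys_Level.
; SwitchActivated increments SwitchesPressed once enough pressure switches are active, and Tick kills the boss at five.
; BeginPlay also starts a TimeToDeath timer leading to its death.
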(event `self.ReceiveBeginPlay`
  (`GameplayStatics.PlaySoundAtLocation` (`self.Sound1`) (`SceneComponent.K2_GetComponentLocation` (`self.Mesh`)) (struct) 1.0 1.0 0.0 null null null null)
  (`KismetSystemLibrary.Delay` (`self.TimeToDeath`))
  ;[1 1 1] plays death anim and sound, and kills actor
  (set `self.Activated` false)
  (`PrimitiveComponent.SetCollisionEnabled` (`self.Mesh`) "NoCollision")
  (`|AIMoveTo` self (0.0 0.0 0.0) self
    (:`then`
      (`GameplayStatics.PlaySoundAtLocation` "/Game/Garnet/Assets/Riley/Sounds/ZombieDeath1_CUE.ZombieDeath1_CUE" (`SceneComponent.K2_GetComponentLocation` (`self.Mesh`)) (struct) 1.0 1.0 0.0 null null null null)
      (`SkeletalMeshComponent.PlayAnimation` (`self.Mesh`) "/Game/Garnet/Assets/Bill/UndeadPack/Lich/Animations/Anim_Death.Anim_Death" false)
      (`KismetSystemLibrary.Delay` 2.0)
      (`self.K2_DestroyActor`))))

(event `self.ReceiveTick`
  (params (DeltaSeconds :type "Float (single-precision)"))
  (if (>= (`self.SwitchesPressed`) 5.0)
    (`GameplayStatics.PlaySoundAtLocation` "/Game/Garnet/Assets/Riley/Sounds/ZombieDeath1_CUE.ZombieDeath1_CUE" (`SceneComponent.K2_GetComponentLocation` (`self.Mesh`)) (struct) 0.8 1.0 0.0 null null null null)
    (`SkeletalMeshComponent.PlayAnimation` (`self.Mesh`) "/Game/Garnet/Assets/Bill/UndeadPack/Lich/Animations/Anim_Death.Anim_Death" false)
    (`KismetSystemLibrary.Delay` 1.5)
    (`self.K2_DestroyActor` self)
    (else
      (`|ExecutionSequence`
        (:`then_0`
          (bind _asbp_devvy (cast `/Game/Blueprints/BP_Devvy` (`GameplayStatics.GetPlayerPawn` 0)))
          (set `self.MinionsAlive` (> (`/Game/Blueprints/BP_Devvy.MinionCount` _asbp_devvy) 0)))
        (:`then_1`
          (`|ExecutionSequence`
            (:`then_0`
              (set `self.DefaultWalkSpeed` (`CharacterMovementComponent.MaxWalkSpeed` (`self.CharacterMovement`)))
              (set `self.DefaultGravity` (`CharacterMovementComponent.GravityScale` (`self.CharacterMovement`))))
            (:`then_1`
              (if (`self.Activated`)
                (if (`self.MinionsAlive`)
                  ;[1 1 1] AI Attack Minions
                  (bind _returnvalue (`GameplayStatics.GetActorOfClass` "/Game/Garnet/Assets/Riley/BP_AI_Minions.BP_AI_Minions_C"))
                  (`|AIMoveTo` self (0.0 0.0 0.0) _returnvalue)
                  (else
                    ;[1 1 1] AI Attack Player
                    (bind _returnvalue_2 (`GameplayStatics.GetActorOfClass` "/Game/Blueprints/BP_Devvy.BP_Devvy_C"))
                    (`|AIMoveTo` self (0.0 0.0 0.0) _returnvalue_2)))))))))))

(event `self.CapsuleComponent.OnComponentHit`
  (params (HitComponent :type "PrimitiveComponent Object Reference") (OtherActor :type "Actor Object Reference") (OtherComp :type "PrimitiveComponent Object Reference") (NormalImpulse :type "Vector Structure") (Hit :type "HitResult Structure (by ref)"))
  (`|ExecutionSequence`
    (:`then_0`
      (bind _asbp_ai_minions (cast `/Game/Garnet/Assets/Riley/BP_AI_Minions` OtherActor))
      (`/Game/Garnet/Assets/Riley/BP_AI_Minions.KillMinionS` _asbp_ai_minions)
      (bind _asbp_devvy (cast `/Game/Blueprints/BP_Devvy` (`GameplayStatics.GetPlayerPawn` 0)))
      (set `/Game/Blueprints/BP_Devvy.MinionCount` (- (`/Game/Blueprints/BP_Devvy.MinionCount` _asbp_devvy) 1) _asbp_devvy))
    (:`then_1`
      (cast `/Game/Blueprints/BP_Devvy` OtherActor)))
  ;[1 1 1] plays death anim and sound, and kills actor
  (set `self.Activated` false)
  (`PrimitiveComponent.SetCollisionEnabled` (`self.Mesh`) "NoCollision")
  (`|AIMoveTo` self (0.0 0.0 0.0) self
    (:`then`
      (`GameplayStatics.PlaySoundAtLocation` "/Game/Garnet/Assets/Riley/Sounds/ZombieDeath1_CUE.ZombieDeath1_CUE" (`SceneComponent.K2_GetComponentLocation` (`self.Mesh`)) (struct) 0.8 1.0 0.0 null null null null)
      (`KismetSystemLibrary.Delay` 1.0)
      (`GameplayStatics.OpenLevel` "Jennys_Level"))))

(event `SwitchActivated`
  (`/Engine/EditorBlueprintResources/StandardMacros.IncrementInt` (`self.PressureSwitchesActive`)
    (:`  `
      (if (>= (`self.PressureSwitchesActive`) (`self.PressureSwitchesNeeded`))
        (`/Engine/EditorBlueprintResources/StandardMacros.IncrementFloat` (`self.SwitchesPressed`)
          (:`  `
            (`GameplayStatics.PlaySoundAtLocation` "/Game/Garnet/Assets/Riley/Sounds/ZombieDeath1_CUE.ZombieDeath1_CUE" (`SceneComponent.K2_GetComponentLocation` (`self.Mesh`)) (struct) 0.8 1.0 0.0 null null null null)))))))

(fn `UserConstructionScript`)